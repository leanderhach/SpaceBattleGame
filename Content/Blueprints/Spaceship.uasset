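; Spaceship prototype of a point-defense system that predicts intercept points for actors inside its DefensePerimeter overlap volume.
; Tick samples tracked actors' transforms twice, separated by delays, and passes each pair to CaclulateTrack.
; That derives range rate and XY angular velocity, then computes a projectile lead point via polar math expressions, with heading and elevation offsets left at zero.
; Output is only debug lines, points and prints; nothing fires.
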(event OnComponentBeginOverlap(DefensePerimeter)
  (params (OverlappedComponent :type Primitive%20Component%20Object%20Reference) (OtherActor :type Actor%20Object%20Reference) (OtherComp :type Primitive%20Component%20Object%20Reference) (OtherBodyIndex :type Integer) (bFromSweep :type Boolean) (SweepResult :type Hit%20Result%20Structure%20%28by%20ref%29))
  (Utilities|Array|Add (Variables|Default|GetTrackedIncoming) OtherActor))

(event OnComponentEndOverlap(DefensePerimeter)
  (params (OverlappedComponent :type Primitive%20Component%20Object%20Reference) (OtherActor :type Actor%20Object%20Reference) (OtherComp :type Primitive%20Component%20Object%20Reference) (OtherBodyIndex :type Integer))
  (Utilities|Array|RemoveItem (Variables|Default|GetTrackedIncoming) OtherActor))

(event EventTick
  (params (DeltaSeconds :type Float%20%28single-precision%29))
  (bind _trackedincoming (Variables|Default|GetTrackedIncoming))
  (bind _incomingplot2 (Variables|Default|GetIncomingPlot2))
  (bind _incomingplot1 (Variables|Default|GetIncomingPlot1))
  (Utilities|FlowControl|Delay 0.5)
  (for _array_element _trackedincoming
    (Utilities|Array|Add _incomingplot1 (Transformation|GetActorTransform _array_element)))
  (Utilities|FlowControl|Delay 0.2)
  (for _array_element_2 _trackedincoming
    (Utilities|Array|Add _incomingplot2 (Transformation|GetActorTransform _array_element_2)))
  (for (_array_element_3 _array_index) _incomingplot1
    (CallFunction|CaclulateTrack _array_element_3 (Utilities|Array|Get(acopy) _incomingplot2 _array_index) (.Location (Math|Transform|BreakTransform (Transformation|GetActorTransform self)))))
  (Utilities|Array|Clear _incomingplot1)
  (Utilities|Array|Clear _incomingplot2))

(fn ConstructionScript)

(fn IncomingObjectTrack
  (params (IncomingObject :type Actor%20Object%20Reference) (DefenseOrigin :type Actor%20Object%20Reference))
  (Development|PrintString (Utilities|String|Append "current: " (Utilities|String|ToString(Vector) (Transformation|GetActorLocation IncomingObject)))))

(fn CaclulateTrack
  (params (InitialLocation :type Transform) (CurrentLocation :type Transform) (DefenseOrigin :type Vector))
  (bind _location (Math|Transform|BreakTransform InitialLocation))
  (bind _location_2 (Math|Transform|BreakTransform CurrentLocation))
  (bind _projectilespeed (Variables|Default|GetProjectileSpeed))
  (bind _pollinginterval (Variables|Default|GetPollingInterval))
  (bind _returnvalue (- _location_2 DefenseOrigin))
  (bind _returnvalue_2 (- _location DefenseOrigin))
  (bind (_x _y _z) (Math|Vector|BreakVector _returnvalue_2))
  (bind (_x_2 _y_2 _z_2) (Math|Vector|BreakVector _returnvalue))
  (bind _returnvalue_3 (Math|Vector|VectorLength _returnvalue))
  (bind (_x_3 _y_3 _z_3) (Math|Vector|BreakVector _returnvalue))
  (bind _returnvalue_4 (Math|Vector|VectorLength _returnvalue_2))
  (bind _returnvalue_5 (- _returnvalue_3 _returnvalue_4))
  (bind _returnvalue_6 (Math|Vector2D|MakeVector2D _x _y))
  (bind _returnvalue_7 (Math|Vector2D|MakeVector2D _x_3 _y_3))
  (bind _returnvalue_8 (/ _returnvalue_5 _pollinginterval))
  (bind _returnvalue_9 (Math|Vector2D|DotProduct(2D) _returnvalue_6 _returnvalue_7))
  (bind _returnvalue_10 (Math|Conversions|ToVector(Vector2D) _returnvalue_6))
  (bind _returnvalue_11 (Math|Conversions|ToVector(Vector2D) _returnvalue_7))
  (bind _returnvalue_12 (Math|Vector|VectorLengthXY _returnvalue_10))
  (bind _returnvalue_13 (Math|Vector|VectorLengthXY _returnvalue_11))
  (bind _returnvalue_14 (|(R/(Vpds-Vm)) _projectilespeed _returnvalue_8 _returnvalue_3))
  (bind _returnvalue_15 (* _returnvalue_12 _returnvalue_13))
  (bind _returnvalue_16 (|(ti*Vpds) _returnvalue_14 _projectilespeed))
  (bind _returnvalue_17 (Math|Float|SafeDivide _returnvalue_9 _returnvalue_15))
  (bind _returnvalue_18 (|((sin(phi))*R) _returnvalue_16 0.0))
  (bind _returnvalue_19 (Math|Trig|Acos(Degrees) _returnvalue_17))
  (bind _returnvalue_20 (/ _returnvalue_19 _pollinginterval))
  (bind _returnvalue_21 (* _returnvalue_20 _returnvalue_14))
  (bind _returnvalue_22 (+ 0.0 _returnvalue_21))
  (bind _returnvalue_23 (|(((cos(theta))*(cos(phi)))*r) _returnvalue_22 _returnvalue_16 0.0))
  (bind _returnvalue_24 (|(((sin(theta))*(cos(phi)))*R) _returnvalue_22 _returnvalue_16 0.0))
  (bind _returnvalue_25 (Math|Vector|MakeVector _returnvalue_23 _returnvalue_24 _returnvalue_18))
  (bind _returnvalue_26 (+ _returnvalue_25 DefenseOrigin))
  (Development|PrintString (Utilities|String|ToString(Float) _x_2))
  (Development|PrintString (Utilities|String|ToString(Float) _y_2))
  (Development|PrintString (Utilities|String|ToString(Float) _z_2))
  (Rendering|Debug|DrawDebugPoint _returnvalue_26 5.0 "(R=1.000000,G=0.000000,B=0.278934,A=1.000000)" 0.5)
  (Rendering|Debug|DrawDebugLine DefenseOrigin _returnvalue_26 "(R=1.000000,G=0.000000,B=0.442750,A=1.000000)" 0.5 1e+01))

(fn CartesiantoPolar
  (params (Point :type Vector))
  (bind (_x _y _z) (Math|Vector|BreakVector Point))
  (return (Math|Vector2D|MakeVector2D (Class|KismetMathLibrary|DegAtan2 (* _z -1.0) (Math|Vector2D|Vector2DLength (Math|Vector2D|MakeVector2D _x _y))) (Class|KismetMathLibrary|DegAtan2 _x _y))))

(fn PolartoCartesian
  (params (Point :type Vector%202D%20Structure))
  (bind _returnvalue (Math|Conversions|ToVector(Vector2D) Point))
  (bind (_x _y) (Math|Vector|BreakVector _returnvalue))
  (return (* (Class|KismetMathLibrary|QuatEuler (Utilities|Struct|MakeQuat _x _y 0.0 1.0)) (Math|Vector|VectorUp))))

(fn Add2Pi
  (params (number :type Float%20%28single-precision%29))
  (return (+ number (* (Math|Trig|GetPI) 2.0))))